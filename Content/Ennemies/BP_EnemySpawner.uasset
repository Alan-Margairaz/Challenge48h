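; Enemy spawner actor that runs growing waves of enemies at random positions around itself.
; A looping timer fires SpawnEnemy, which picks from four EnemiesRandomiser classes using rerolls per branch, so odds are uneven and some ticks spawn nothing.
; Reaching the wave quota pauses the timer.
; CheckAmountOfEnnemiesKilled resets counters, raises the quota and resumes the same timer once kills, counted outside this graph, reach the quota.
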(event `CheckAmountOfEnnemiesKilled`
  ;[1 1 1] Waves Reset + Increment
  (if (>= (`self.AmountKilled`) (`self.AmountsToSpawn`))
    (`KismetSystemLibrary.PrintString` "True")
    (set `self.AmountThatSpawned` 0)
    (set `self.AmountKilled` 0)
    (set `self.AmountsToSpawn` (+ (`self.AmountsToSpawn`) 3))
    (`KismetSystemLibrary.PrintString` "Reset done")
    ;[1 1 1] Timer Pause Between Waves
    (`KismetSystemLibrary.K2_UnPauseTimerHandle` (`self.EnemySpawnTimer`))
    (`KismetSystemLibrary.PrintString` "Spawn faster")))

(event `SpawnEnemy`
  (bind (_returnvalue_x _returnvalue_y _returnvalue_z) (`KismetMathLibrary.BreakVector` (`self.K2_GetActorLocation`)))
  (bind _returnvalue (`KismetMathLibrary.RandomIntegerInRange` 0 100))
  ;[1 1 1] Random Localization Spawner
  (bind _output_get (set `self.EnemySpawnLocation` (`KismetMathLibrary.MakeVector` (+ (`KismetMathLibrary.RandomFloatInRange` -700.0 700.0) _returnvalue_x) (+ (`KismetMathLibrary.RandomFloatInRange` -700.0 700.0) _returnvalue_y) (+ _returnvalue_z (`KismetMathLibrary.RandomFloatInRange` -300.0 300.0)))))
  ;[1 1 1] Enemy Randomizer
  (if (<= _returnvalue 25)
    (bind _returnvalue_2 (`KismetMathLibrary.Conv_VectorToTransform` _output_get))
    (`|SpawnActorFromClass` (`|GetArrayItem` (`self.EnemiesRandomiser`)) _returnvalue_2 "AdjustIfPossibleButDontSpawnIfColliding" "OverrideRootScale" null null)
    (`KismetSystemLibrary.PrintString` "25%")
    ;[1 1 1] Wave behavior
    (bind _result (`/Engine/EditorBlueprintResources/StandardMacros.IncrementInt` (`self.AmountThatSpawned`) :!label _label)
      (:`  `
        (if (>= _result (`self.AmountsToSpawn`))
          (`KismetSystemLibrary.K2_PauseTimerHandle` (`self.EnemySpawnTimer`)))))
    (elif (and (> _returnvalue 25) (<= _returnvalue 50))
      (`|SpawnActorFromClass` (`|GetArrayItem` (`self.EnemiesRandomiser`) 1) _returnvalue_2 "AdjustIfPossibleButDontSpawnIfColliding" "OverrideRootScale" null null)
      (`KismetSystemLibrary.PrintString` "50%")
      (goto _label)
      (elif (<= _returnvalue 75)
        (`|SpawnActorFromClass` (`|GetArrayItem` (`self.EnemiesRandomiser`) 2) _returnvalue_2 "AdjustIfPossibleButDontSpawnIfColliding" "OverrideRootScale" null null)
        (`KismetSystemLibrary.PrintString` "75%")
        (goto _label)
        (elif (> _returnvalue 75)
          (`|SpawnActorFromClass` (`|GetArrayItem` (`self.EnemiesRandomiser`) 3) _returnvalue_2 "AdjustIfPossibleButDontSpawnIfColliding" "OverrideRootScale" null null)
          (`KismetSystemLibrary.PrintString` "100%")
          (goto _label))))))

(event `self.ReceiveBeginPlay`
  ;[1 1 1] Random Localization Spawner
  (bind _returnvalue (`KismetSystemLibrary.K2_SetTimerDelegate` (delegate `SpawnEnemy`) 1.0 true))
  (set `self.EnemySpawnTimer` _returnvalue))

(fn `UserConstructionScript`)